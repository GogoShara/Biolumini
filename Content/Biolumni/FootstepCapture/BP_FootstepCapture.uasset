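; Scene-capture actor that follows the player and records footsteps into a persistent render target.
; Each tick it moves by whole-texel steps (ortho width over 256) to avoid swimming, then publishes its location to MPC_Footsteps.
; A dynamic draw material receives that move as a UV-space offset and draws into RT_PersistentFootsteps to keep the trail aligned.
; CaptureOffset receives player velocity, which is also debug-printed.
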(event EventTick
  (params (DeltaSeconds :type Float%20%28single-precision%29))
  (CallFunction|MoveCapture)
  (CallFunction|DrawtoPersistent))

(event EventBeginPlay
  (Rendering|Material|SetScalarParameterValue "/Game/Biolumni/FootstepCapture/MPC_Footsteps.MPC_Footsteps" "CaptureSize" (Variables|/Script/Engine.SceneCaptureComponent2D|GetOrthoWidth (Variables|Default|GetSceneCaptureComponent2D)) :!class /Script/Engine.KismetMaterialLibrary)
  (bind _returnvalue (Rendering|Material|CreateDynamicMaterialInstance "/Game/Biolumni/FootstepCapture/M_DrawToPersistent.M_DrawToPersistent" "None" "None" :!class /Script/Engine.KismetMaterialLibrary))
  (Variables|Default|SetDrawMaterial _returnvalue)
  (Rendering|ClearRenderTarget2D "/Game/Biolumni/FootstepCapture/RT_Footsteps.RT_Footsteps")
  (Rendering|ClearRenderTarget2D "/Game/Biolumni/FootstepCapture/RT_PersistentFootsteps.RT_PersistentFootsteps"))

(fn ConstructionScript)

(fn MoveCapture
  (bind _returnvalue (Game|GetPlayerCharacter 0))
  (bind _returnvalue_2 (Game|GetPlayerCharacter 0))
  (bind _returnvalue_3 (/ 1.0 256.0))
  (bind _returnvalue_4 (Transformation|GetActorLocation))
  (bind _scenecapturecomponent2d (Variables|Default|GetSceneCaptureComponent2D))
  (bind _returnvalue_5 (Transformation|GetActorLocation _returnvalue_2))
  (bind _returnvalue_6 (Transformation|GetVelocity _returnvalue))
  (bind _orthowidth (Variables|/Script/Engine.SceneCaptureComponent2D|GetOrthoWidth _scenecapturecomponent2d))
  (bind _returnvalue_7 (* _orthowidth _returnvalue_3))
  (bind _returnvalue_8 (CallFunction|SnaptoPixelWorldSize (.x _returnvalue_5) (.y _returnvalue_5) _returnvalue_7))
  (bind _returnvalue_9 (- _returnvalue_8 _returnvalue_4))
  (Utilities|IsValid _returnvalue_2
    (:Is%20Valid
      (bind _output_get (Variables|Default|SetMove%20Offset (Math|Vector2D|MakeVector2D (.x _returnvalue_9) (.y _returnvalue_9))))
      (Rendering|Material|SetVectorParameterValue "/Game/Biolumni/FootstepCapture/MPC_Footsteps.MPC_Footsteps" "CaptureOffset" (Math|Conversions|ToLinearColor(Vector) _returnvalue_6) :!class /Script/Engine.KismetMaterialLibrary)
      (Development|PrintString (Utilities|String|ToString(Integer) (Math|Conversions|ToLinearColor(Vector) _returnvalue_6)))
      (Transformation|AddActorWorldOffset (Math|Vector|MakeVector (.x _output_get) (.y _output_get) 0.0))
      (Rendering|Material|SetVectorParameterValue "/Game/Biolumni/FootstepCapture/MPC_Footsteps.MPC_Footsteps" "CaptureLocation" (Math|Conversions|ToLinearColor(Vector) (Transformation|GetActorLocation)) :!class /Script/Engine.KismetMaterialLibrary))))

(fn SnaptoPixelWorldSize
  (params (PlayerX :type Float%20%28double-precision%29) (PlayerY :type Float%20%28double-precision%29) (PixelWorldSize :type Float%20%28double-precision%29))
  (return (|(((vector((floor((PlayerX/PixelWorldSize))),(floor((PlayerY/PixelWorldSize))),0))+0.500000)*PixelWorldSize) PlayerX PlayerY PixelWorldSize)))

(fn DrawtoPersistent
  (bind _move_offset (Variables|Default|GetMove%20Offset))
  (bind _scenecapturecomponent2d (Variables|Default|GetSceneCaptureComponent2D))
  (bind _orthowidth (Variables|/Script/Engine.SceneCaptureComponent2D|GetOrthoWidth _scenecapturecomponent2d))
  (bind _returnvalue (/ _move_offset _orthowidth))
  (Rendering|Material|SetVectorParameterValue (Variables|Default|GetDrawMaterial) "Offset" (Utilities|Struct|MakeLinearColor (.x _returnvalue) (.y _returnvalue) 0.0 1.0) :!class /Script/Engine.MaterialInstanceDynamic)
  (Rendering|DrawMaterialtoRenderTarget "/Game/Biolumni/FootstepCapture/RT_PersistentFootsteps.RT_PersistentFootsteps" (Variables|Default|GetDrawMaterial)))